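; Game mode for a point-collection game with levels, enemies and a victory screen.
; On start it creates the HUD, caches a RespawnBox's bounds and spawns a PointBall at a random point inside them.
; Respawn spawns and possesses a new character in that box.
; Addpoint counts points down, raises level and quota at zero, and either spawns another actor plus an enemy or, after the final level, shows victory and pauses.
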(event `self.ReceiveBeginPlay`
  ;[1 1 1] Inicializar BasicHUD
  (bind _returnvalue (`|CreateWidget` "/Game/UI/BasicHUD.BasicHUD_C"))
  (bind _output_get (set `self.HUD` _returnvalue))
  (`UserWidget.AddToViewport` _output_get 0)
  (bind _outactors (`GameplayStatics.GetAllActorsOfClass` "/Game/Levels/RespawnBox.RespawnBox_C"))
  (bind (_origin _boxextent) (`self.GetActorBounds` (`|GetArrayItem` _outactors) false false))
  (set `self.Origin` _origin)
  (set `self.Box Extent` _boxextent)
  (`|SpawnActorFromClass` "/Game/Levels/PointBall.PointBall_C" (`KismetMathLibrary.MakeTransform` (`KismetMathLibrary.RandomPointInBoundingBox` (`self.Origin`) (`self.Box Extent`))) "AdjustIfPossibleButAlwaysSpawn" "OverrideRootScale" null null))

(event `Respawn`
  (params (Character :type "Character Object Reference"))
  ;[1 1 1] Recoloar Jugador
  (bind _returnvalue (`|SpawnActorFromClass` (`GameplayStatics.GetObjectClass` Character) (`KismetMathLibrary.MakeTransform` (`KismetMathLibrary.RandomPointInBoundingBox` (`self.Origin`) (`self.Box Extent`))) "AdjustIfPossibleButAlwaysSpawn" "OverrideRootScale" null null))
  (`Controller.Possess` (`GameplayStatics.GetPlayerController` 0) _returnvalue))

(event `Addpoint`
  (bind _box_extent (`self.Box Extent`))
  (bind _origin (`self.Origin`))
  (bind _hud (`self.HUD`))
  ;[1 1 1] Reducir Puntos + Subir nivel si es necesario + Victoria
  (bind _output_get (set `self.Point` (- (`self.Point`) 1)))
  (if (<= _output_get 0)
    (bind _result (`/Engine/EditorBlueprintResources/StandardMacros.IncrementInt` (`self.Level`))
      (:`  `
        (if (>= _result 3)
          ;[1 1 1] Victoria
          (`Widget.SetVisibility` (`/Game/UI/BasicHUD.VictoryText` (`self.HUD`)) "Visible")
          (`GameplayStatics.SetGamePaused` true)
          (else
            (bind _output_get_2 (set `self.Point` (* _result 5)))
            (set `/Game/UI/BasicHUD.Nivel` _result _hud)
            (set `/Game/UI/BasicHUD.Points` _output_get_2 _hud)
            (`|SpawnActorFromClass` "/Game/Levels/PointBall.PointBall_C" (`KismetMathLibrary.MakeTransform` (`KismetMathLibrary.RandomPointInBoundingBox` _origin _box_extent)) "AdjustIfPossibleButAlwaysSpawn" "OverrideRootScale" null null :!label _label)
            (`|SpawnActorFromClass` "/Game/Characters/Enemy/BP_Enemy/BP_enemy.BP_enemy_C" (`KismetMathLibrary.MakeTransform` (`KismetMathLibrary.RandomPointInBoundingBox` _origin _box_extent)) "AdjustIfPossibleButAlwaysSpawn" "OverrideRootScale" null null)))))
    (else
      (set `/Game/UI/BasicHUD.Points` _output_get _hud)
      (goto _label))))

(fn `UserConstructionScript`)